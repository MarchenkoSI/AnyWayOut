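; Game mode for an anomaly-spotting floor loop, with mouse-sensitivity saving and an exit achievement on finishing.
; It builds the level endlessly by spawning and destroying main sections and two exit transitions as the player moves.
; Each main section rolls a weighted anomaly chance, which decides the correct exit.
; Correct choices lower the floor counter toward the final floor-zero section, while wrong ones reset it to ten.
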(event Custom|HandlePlayerEnterTransition
  (params (Transition :type P%20Transition%20Object%20Reference))
  (Variables|Default|SetIsEnterMain false)
  (Default|DestroyAnomalyifNeeded (Variables|Default|GetCurrentMainSection))
  (Actor|DestroyActor (Variables|Default|GetCurrentMainSection))
  (CallFunction|CheckPlayerChoice Transition)
  (if (== (Variables|Default|GetCurrentFloor) 0)
    (bind _transform (Default|GetNewMainSectionSpawnTransform Transition))
    (Game|SpawnActorfromClass "/Game/AnyWayOut/Prefabs/P_0_Floor.P_0_Floor_C" _transform "Undefined" 0 0)
    (else
      (bind _transform_2 (Default|GetNewMainSectionSpawnTransform Transition))
      (bind _returnvalue (Game|SpawnActorfromClass "/Game/AnyWayOut/Prefabs/Prefab_MainSection.Prefab_MainSection_C" _transform_2 "Undefined" 0 0))
      (bind _output_get (Variables|Default|SetCurrentMainSection _returnvalue))
      (Variables|/Game/AnyWayOut/Prefabs/Prefab_MainSection.Prefab_MainSection_C|SetIsActive _output_get false)
      (Default|OnCreated (Variables|Default|GetCurrentMainSection)))))

(event Custom|HandlePlayerEnterMain
  (if (not (Variables|Default|GetIsEnterMain))
    (Variables|Default|SetIsEnterMain true)
    (CallFunction|DestroyTransitionSection (Variables|Default|GetCurrentTransitionOne))
    (CallFunction|DestroyTransitionSection (Variables|Default|GetCurrentTransitionTwo))
    (bind _newparam (Default|GetExitOneTransform (Variables|Default|GetCurrentMainSection)))
    (bind _returnvalue (Game|SpawnActorfromClass "/Game/AnyWayOut/Prefabs/P_Transition.P_Transition_C" _newparam "Undefined" 0 0))
    (Variables|Default|SetCurrentTransitionTwo _returnvalue)
    (bind _newparam_2 (Default|GetExitTwoTransform (Variables|Default|GetCurrentMainSection)))
    (bind _returnvalue_2 (Game|SpawnActorfromClass "/Game/AnyWayOut/Prefabs/P_Transition.P_Transition_C" _newparam_2 "Undefined" 0 0))
    (Variables|Default|SetCurrentTransitionOne _returnvalue_2)
    (bind _anomalyneeded (CallFunction|PrepareAnomaly))
    (bind _output_get (Variables|Default|SetWithAnomaly _anomalyneeded))
    (Default|UpdateAnomaly (Variables|Default|GetCurrentMainSection) _output_get)
    (bind _returnvalue_3 (Actor|GetActorOfClass "/Script/NavigationSystem.NavMeshBoundsVolume"))
    (Variables|Default|SetNavMesh _returnvalue_3)))

(event Custom|GameFinished
  (bind _returnvalue (Actor|GetActorOfClass "/Game/AnyWayOut/Blueprints/BP_Player.BP_Player_C"))
  (if (Utilities|IsValid _returnvalue)
    (Default|ShowFinal _returnvalue)
    (|CacheAchievements (Game|GetPlayerController 0)
      (:OnSuccess
        (bind (_bfoundid _progress) (Class|AchievementBlueprintLibrary|GetCachedAchievementProgress (Game|GetPlayerController 0) "Achievement_01_Exit"))
        (if _bfoundid
          (if (not (> _progress 0.0))
            (|WriteAchievementProgress (Game|GetPlayerController 0) "Achievement_01_Exit" 1e+02)))))))

(event Custom|HandleFinalFloorEnter
  (bind _outactors (Actor|GetAllActorsOfClass "/Game/AnyWayOut/Prefabs/P_Door.P_Door_C"))
  (for _array_element _outactors
    (Default|ForceClose _array_element)))

(event Custom|Restart
  (Development|ExecuteConsoleCommand "RestartLevel" 0))

(event Custom|ProcessingAnomalyList
  (params (AnomalyIndex :type Integer))
  (Utilities|Array|Add (Variables|Default|GetUsedAnomalyIndex) AnomalyIndex)
  (if (>= (Utilities|Array|Length (Variables|Default|GetUsedAnomalyIndex)) 20)
    (Utilities|Array|Clear (Variables|Default|GetUsedAnomalyIndex))))

(event EventBeginPlay
  (CallFunction|LoadGame "0")
  (CallFunction|SaveGame "0")
  (bind _returnvalue (Game|SpawnActorfromClass "/Game/AnyWayOut/Prefabs/Prefab_MainSection.Prefab_MainSection_C" (Transformation|GetWorldTransform (Variables|Default|GetDefaultSceneRoot)) "Undefined" 0 0))
  (bind _output_get (Variables|Default|SetCurrentMainSection _returnvalue))
  (Variables|/Game/AnyWayOut/Prefabs/Prefab_MainSection.Prefab_MainSection_C|SetIsActive _output_get true)
  (Default|OnCreated (Variables|Default|GetCurrentMainSection))
  (bind _newparam (Default|GetExitOneTransform (Variables|Default|GetCurrentMainSection)))
  (bind _returnvalue_2 (Game|SpawnActorfromClass "/Game/AnyWayOut/Prefabs/P_Transition.P_Transition_C" _newparam "Undefined" 0 0))
  (Variables|Default|SetCurrentTransitionOne _returnvalue_2)
  (bind _newparam_2 (Default|GetExitTwoTransform (Variables|Default|GetCurrentMainSection)))
  (bind _returnvalue_3 (Game|SpawnActorfromClass "/Game/AnyWayOut/Prefabs/P_Transition.P_Transition_C" _newparam_2 "Undefined" 0 0))
  (Variables|Default|SetCurrentTransitionTwo _returnvalue_3)
  (Variables|Default|SetCurrentFloor 1)
  (bind _returnvalue_4 (Settings|GetGameUserSettings))
  (Class|GameUserSettings|SetVSyncEnabled _returnvalue_4 true)
  (Class|GameUserSettings|ApplyNonResolutionSettings _returnvalue_4))

(fn ConstructionScript)

(fn LoadGame
  (params (SlotName :type String))
  (bind _returnvalue (SaveGame|DoesSaveGameExist SlotName))
  (if _returnvalue
    (bind _returnvalue_2 (SaveGame|LoadGamefromSlot SlotName))
    (bind _asbp_saver (Utilities|Casting|CastToBP_Saver _returnvalue_2))
    (Variables|Default|SetMouseSens (Variables|/Game/AnyWayOut/Blueprints/BP_Saver.BP_Saver_C|GetMouseSens _asbp_saver))))

(fn SaveGame
  (params (SlotName :type String))
  (bind _returnvalue (SaveGame|DoesSaveGameExist SlotName))
  (if _returnvalue
    (bind _returnvalue_2 (SaveGame|LoadGamefromSlot SlotName))
    (Variables|Default|SetSave_REF _returnvalue_2)
    (else
      (bind _returnvalue_3 (SaveGame|CreateSaveGameObject "/Game/AnyWayOut/Blueprints/BP_Saver.BP_Saver_C"))
      (bind _output_get (Variables|Default|SetSave_REF _returnvalue_3))))
  (bind _asbp_saver (Utilities|Casting|CastToBP_Saver _output_get))
  (Variables|/Game/AnyWayOut/Blueprints/BP_Saver.BP_Saver_C|SetMouseSens _asbp_saver (Variables|Default|GetMouseSens))
  (SaveGame|SaveGametoSlot (Variables|Default|GetSave_REF) SlotName))

(fn CheckPlayerChoice
  (params (EnterTransition :type P%20Transition%20Object%20Reference))
  (if (Variables|Default|GetFirstChoice)
    (Variables|Default|SetFirstChoice false)
    (if (== (Variables|Default|GetCurrentTransitionTwo) EnterTransition)
      (Variables|Default|SetCurrentFloor (- (Variables|Default|GetCurrentFloor) 1) :!label _label)
      (else
        (Variables|Default|SetCurrentFloor 10 :!label _label_2)))
    (elif (Variables|Default|GetWithAnomaly)
      (if (== EnterTransition (Variables|Default|GetCurrentTransitionTwo))
        (goto _label)
        (else
          (goto _label_2)))
      (elif (== EnterTransition (Variables|Default|GetCurrentTransitionOne))
        (goto _label)
        (else
          (goto _label_2))))))

(fn DestroyTransitionSection
  (params (Transtion :type P%20Transition%20Object%20Reference))
  (Actor|DestroyActor (Variables|/Game/AnyWayOut/Prefabs/P_Transition.P_Transition_C|GetDoor_UP Transtion))
  (Actor|DestroyActor Transtion))

(fn PrepareAnomaly
  (return (Math|Random|RandomBoolwithWeight 0.6)))

(fn GetGameMode
  (return self))