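; First-person player character for AnyWayOut, handling movement, sprinting, mouse look and line-trace interaction from the camera.
; BeginPlay runs a fade-in overlay before enabling control, and ShowFinal fades in an ending screen, scrolls credits, then restarts through the game mode.
; It also toggles the pause menu, switches its spotlight on or off, and can teleport itself to a fixed floor height.
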(event Custom|HidePause
  (bind _returnvalue (Game|GetPlayerController 0))
  (Widget|RemovefromParent (Variables|Default|GetPauseOverlay))
  (Input|SetInputModeGameOnly _returnvalue)
  (Variables|/Script/Engine.PlayerController|SetbShowMouseCursor _returnvalue false)
  (Variables|Default|SetPauseMenuOpened false)
  (Variables|Default|SetCanMove true))

(event Custom|TurnLight
  (params (Value :type Boolean))
  (bind _spotlight (Variables|Default|GetSpotLight))
  (if Value
    (Rendering|Components|Light|SetIntensity _spotlight 2.5e+02)
    (else
      (Rendering|Components|Light|SetIntensity _spotlight 0.0))))

(event Custom|ShowFinal
  (Variables|Default|SetCanMove false)
  (Variables|Default|SetGameStarted false)
  (bind _playercontroller (Class|INTPlayerController|GetPlayerControllerRef(Message) (Pawn|GetController)))
  (bind _returnvalue (UserInterface|CreateWidget "/Game/AnyWayOut/Blueprints/UI/FinalWidget.FinalWidget_C" _playercontroller))
  (bind _output_get (Variables|Default|SetFinalOverlay _returnvalue))
  (UserInterface|Viewport|AddtoViewport _output_get 0)
  (bind _newtrack_0 (Timeline|Timeline_0 Play)
    (:Update
      (Default|SetImageColor (Variables|Default|GetFinalOverlay) _newtrack_0))
    (:Finished
      (bind _newtrack_0_2 (Timeline|Credits Play)
        (:Update
          (Default|MoveCredits (Variables|Default|GetFinalOverlay) _newtrack_0_2))
        (:Finished
          (Utilities|FlowControl|Delay 5.0)
          (bind _gamemode (Class|INTGameMode|GetGameMode(Message) (Game|GetGameMode)))
          (Default|Restart _gamemode))))))

(event Custom|TeleportToZero
  (bind _capsulecomponent (Variables|Collision|GetCapsuleComponent))
  (bind _capsulecomponent_2 (Variables|Collision|GetCapsuleComponent))
  (bind _capsulecomponent_3 (Variables|Collision|GetCapsuleComponent))
  (bind _returnvalue (Transformation|GetWorldLocation _capsulecomponent_2))
  (Physics|SetEnableGravity _capsulecomponent_3 false)
  (Collision|SetCollisionEnabled _capsulecomponent_3 "NoCollision")
  (Transformation|SetActorLocation self (Math|Vector|MakeVector (.x _returnvalue) (.y _returnvalue) 90.150116) false false)
  (Collision|SetCollisionEnabled _capsulecomponent "QueryAndPhysics")
  (Physics|SetEnableGravity _capsulecomponent true))

(event EventBeginPlay
  (bind _playercontroller (Class|INTPlayerController|GetPlayerControllerRef(Message) (Pawn|GetController)))
  (bind _returnvalue (UserInterface|CreateWidget "/Game/AnyWayOut/Blueprints/UI/InitWidget.InitWidget_C" _playercontroller))
  (bind _output_get (Variables|Default|SetInitOverlay _returnvalue))
  (UserInterface|Viewport|AddtoViewport _output_get 0)
  (bind _value (Timeline|Fade Play)
    (:Update
      (Default|SetImageColor (Variables|Default|GetInitOverlay) _value))
    (:Finished
      (Variables|Default|SetCanMove true)
      (Widget|RemovefromParent (Variables|Default|GetInitOverlay))
      (Variables|Default|SetGameStarted true))))

(event Input|ActionEvents|InputActionIA_Run
  (params (Key :type Key%20Structure :default "None"))
  (bind _charactermovement (Variables|Character|GetCharacterMovement))
  (:Pressed
    (Variables|/Script/Engine.CharacterMovementComponent|SetMaxWalkSpeed _charactermovement 4e+02))
  (:Released
    (Variables|/Script/Engine.CharacterMovementComponent|SetMaxWalkSpeed _charactermovement 2e+02)))

(event Input|ActionEvents|InputActionIA_Interact
  (params (Key :type Key%20Structure :default "None"))
  (:Pressed
    (if (Variables|Default|GetCanMove)
      (if (Variables|Default|GetInteractReleased)
        (Variables|Default|SetInteractReleased false)
        (CallFunction|FInteract))))
  (:Released
    (Variables|Default|SetInteractReleased true)))

(event Input|ActionEvents|InputActionIA_Pause
  (params (Key :type Key%20Structure :default "None"))
  (bind _returnvalue (Game|GetPlayerController 0))
  (bind _returnvalue_2 (Game|GetPlayerController 0))
  (:Pressed
    (if (Variables|Default|GetGameStarted)
      (if (Variables|Default|GetPauseMenuOpened)
        (Widget|RemovefromParent (Variables|Default|GetPauseOverlay))
        (Input|SetInputModeGameOnly _returnvalue)
        (Variables|/Script/Engine.PlayerController|SetbShowMouseCursor _returnvalue false)
        (Variables|Default|SetPauseMenuOpened false)
        (Variables|Default|SetCanMove true)
        (else
          (bind _returnvalue_3 (UserInterface|CreateWidget "/Game/AnyWayOut/Blueprints/UI/PauseWidget.PauseWidget_C" _returnvalue))
          (bind _output_get (Variables|Default|SetPauseOverlay _returnvalue_3))
          (UserInterface|Viewport|AddtoViewport _output_get 0)
          (Input|SetInputModeGameandUI _returnvalue_2 (Variables|Default|GetPauseOverlay) "DoNotLock" true)
          (Variables|/Script/Engine.PlayerController|SetbShowMouseCursor _returnvalue_2 true)
          (Variables|Default|SetPauseMenuOpened true)
          (Variables|Default|SetCanMove false))))))

(event Input|AxisEvents|InputAxisIA_Forward
  (params (AxisValue :type Float%20%28single-precision%29))
  (if (Variables|Default|GetCanMove)
    (Pawn|Input|AddMovementInput (Transformation|GetActorForwardVector) AxisValue false)))

(event Input|AxisEvents|InputAxisIA_Backward
  (params (AxisValue :type Float%20%28single-precision%29))
  (if (Variables|Default|GetCanMove)
    (Pawn|Input|AddMovementInput (Transformation|GetActorForwardVector) (* -1 AxisValue) false)))

(event Input|AxisEvents|InputAxisIA_Rigth
  (params (AxisValue :type Float%20%28single-precision%29))
  (if (Variables|Default|GetCanMove)
    (Pawn|Input|AddMovementInput (Transformation|GetActorRightVector) AxisValue false)))

(event Input|AxisEvents|InputAxisIA_Left
  (params (AxisValue :type Float%20%28single-precision%29))
  (if (Variables|Default|GetCanMove)
    (Pawn|Input|AddMovementInput (Transformation|GetActorRightVector) (* -1 AxisValue) false)))

(event Input|MouseEvents|Mouse2D
  (params (AxisValue :type Vector :default "0, 0, 0"))
  (if (Variables|Default|GetCanMove)
    (bind _gamemode (Class|INTGameMode|GetGameMode(Message) (Game|GetGameMode)))
    (Pawn|Input|AddControllerYawInput (* (Variables|/Game/AnyWayOut/Blueprints/BP_GameMode.BP_GameMode_C|GetMouseSens _gamemode) (.x AxisValue)))
    (Pawn|Input|AddControllerPitchInput (* -1 (* (Variables|/Game/AnyWayOut/Blueprints/BP_GameMode.BP_GameMode_C|GetMouseSens _gamemode) (.y AxisValue))))))

(fn ConstructionScript)

(fn FInteract
  (bind _camera (Variables|Default|GetCamera))
  (bind _returnvalue (Transformation|GetWorldLocation _camera))
  (if (Variables|Default|GetCanMove)
    (bind _outhit (Collision|LineTraceByChannel _returnvalue (+ _returnvalue (* (Math|Vector|GetForwardVector _camera) 200)) "TraceTypeQuery1" false 0 "None"))
    (Class|INTInteract|Interact(Message) (.HitActor (Collision|BreakHitResult _outhit)))))

(fn GetPlayerRef
  (return self))